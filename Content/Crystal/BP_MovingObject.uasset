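; BP_MovingObject is a collectible crystal pickup that floats and spins in place until the player touches it.
; After a random start delay, which staggers instances, a Timeline drives the mesh's relative height and yaw.
; When the Capsule overlaps BP_ThirdPersonCharacter, it increments that character's CrystalsCollector count, plays a coin sound, spawns a particle effect and destroys itself.
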(event `self.ReceiveBeginPlay`
  ;[0 0.4173 1] Crystal Movement
  (`KismetSystemLibrary.Delay` (`KismetMathLibrary.RandomFloatInRange` 0.0 2.0))
  (bind (_direction _height _spin) (`Timeline|Timeline`)
    (:`Update`
      (`SceneComponent.K2_SetRelativeLocationAndRotation` (`self.StaticMesh`) (`KismetMathLibrary.MakeVector` 0.0 0.0 _height) (`KismetMathLibrary.MakeRotator` 0.0 0.0 _spin) false false))))

(event `self.Capsule.OnComponentBeginOverlap`
  (params (OverlappedComponent :type "PrimitiveComponent Object Reference") (OtherActor :type "Actor Object Reference") (OtherComp :type "PrimitiveComponent Object Reference") (OtherBodyIndex :type Integer) (bFromSweep :type Boolean) (SweepResult :type "HitResult Structure (by ref)"))
  ;[1 0 0] Destroy on collision
  (bind _asbp_third_person_character (cast `/Game/ThirdPerson/Blueprints/BP_ThirdPersonCharacter` OtherActor))
  (bind _result (`/Engine/EditorBlueprintResources/StandardMacros.IncrementInt` (`/Game/ThirdPerson/Blueprints/BP_ThirdPersonCharacter.CrystalsCollector` _asbp_third_person_character))
    (:`  `
      (set `/Game/ThirdPerson/Blueprints/BP_ThirdPersonCharacter.CrystalsCollector` _result _asbp_third_person_character)
      (`GameplayStatics.PlaySound2D` "/Game/GAME_COINS_SFX_PACK1/GAME_COINS_SFX_T2_P1-98_Cue.GAME_COINS_SFX_T2_P1-98_Cue" 1.0 1.0 0.0 null null)
      (`NiagaraFunctionLibrary.SpawnSystemAtLocation` "/Game/Crystal/Particles.Particles" (`self.K2_GetActorLocation`))
      (`self.K2_DestroyActor`))))

(fn `UserConstructionScript`)